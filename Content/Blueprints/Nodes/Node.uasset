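; Node is a placeable marker actor that displays configurable text, which turns every tick to face the first player's pawn.
; Its construction script snaps it onto nearby geometry with debug-drawn line traces, first upward, then downward from the resulting position.
; The same script enables the collider only when the node is flagged as a target node.
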(event EventTick
  (params (DeltaSeconds :type Float%20%28single-precision%29))
  (Transformation|SetWorldRotation (Variables|Default|GetRepresentation) (Math|Rotator|FindLookatRotation (Transformation|GetActorLocation) (Transformation|GetActorLocation (Pawn|GetControlledPawn (Game|GetPlayerController 0)))) false false))

(event EventBeginPlay
  (Rendering|Components|TextRender|SetText (Variables|Default|GetRepresentation) (Variables|Default|GetTextToDisplay)))

(fn ConstructionScript
  (bind _returnvalue (Transformation|GetActorLocation))
  (bind _returnvalue_2 (Transformation|GetActorLocation))
  (bind _collider (Variables|Default|GetCollider))
  (Utilities|FlowControl|Sequence
    (:then_0
      (bind (_outhit _returnvalue_3) (Collision|LineTraceByChannel _returnvalue (+ _returnvalue "0, 0,1000.000000") "TraceTypeQuery5" false 0 "ForDuration" true "(R=1.000000,G=0.000000,B=0.000000,A=1.000000)" "(R=0.000000,G=1.000000,B=0.000000,A=1.000000)" 2.0))
      (if _returnvalue_3
        (Transformation|SetActorLocation (.Location (Collision|BreakHitResult _outhit)) false false)))
    (:then_1
      (bind (_outhit_2 _returnvalue_4) (Collision|LineTraceByChannel _returnvalue_2 (+ _returnvalue_2 "0, 0,-1000.000000") "TraceTypeQuery5" false 0 "ForDuration" true "(R=1.000000,G=0.000000,B=0.000000,A=1.000000)" "(R=0.000000,G=1.000000,B=0.000000,A=1.000000)" 2.0))
      (if _returnvalue_4
        (Transformation|SetActorLocation (.Location (Collision|BreakHitResult _outhit_2)) false false)))
    (:then_2
      (if (Variables|Default|GetIsTargetNode)
        (Collision|SetCollisionEnabled _collider "QueryAndPhysics")
        (else
          (Collision|SetCollisionEnabled _collider "NoCollision"))))))