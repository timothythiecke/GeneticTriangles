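; Terrain actor that provides a configurable noise-based ground mesh in five difficulty tiers, from Base to Extremely Harsh.
; All setup runs in the construction script, which scales the actor uniformly in X and Y and picks a noise mesh from the terrain type.
; The same mesh goes to a Representation component and a Hidden component, the latter offset along Z with configurable in-game visibility.
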(event EventBeginPlay)

(event Collision|EventActorBeginOverlap
  (params (OtherActor :type Actor%20Object%20Reference)))

(event EventTick
  (params (DeltaSeconds :type Float%20%28single-precision%29)))

(fn ConstructionScript
  (bind _desiredscale (Variables|Default|GetDesiredScale))
  (bind _hidden (Variables|Default|GetHidden))
  (Transformation|SetActorScale3D (Math|Vector|MakeVector _desiredscale _desiredscale 1.0))
  (Transformation|SetRelativeLocation (Variables|Default|GetHidden) (Math|Vector|MakeVector 0.0 0.0 (Variables|Default|GetDesiredDistanceOfHiddenTerrain)) false false)
  (Development|SetHiddeninGame (Variables|Default|GetHidden) (Variables|Default|GetIsHidden) false)
  (switch Utilities|FlowControl|Switch|SwitchonETerrainType (Variables|Default|GetTerrainType)
    (:NewEnumerator0
      (Components|StaticMesh|SetStaticMesh (Variables|Default|GetRepresentation) "/Game/Meshes/Noise25.Noise25")
      (Components|StaticMesh|SetStaticMesh _hidden "/Game/Meshes/Noise25.Noise25"))
    (:NewEnumerator1
      (Components|StaticMesh|SetStaticMesh (Variables|Default|GetRepresentation) "/Game/Meshes/Noise50.Noise50")
      (Components|StaticMesh|SetStaticMesh _hidden "/Game/Meshes/Noise50.Noise50"))
    (:NewEnumerator2
      (Components|StaticMesh|SetStaticMesh (Variables|Default|GetRepresentation) "/Game/Meshes/Noise75.Noise75")
      (Components|StaticMesh|SetStaticMesh _hidden "/Game/Meshes/Noise75.Noise75"))
    (:NewEnumerator3
      (Components|StaticMesh|SetStaticMesh (Variables|Default|GetRepresentation) "/Game/Meshes/Noise100.Noise100")
      (Components|StaticMesh|SetStaticMesh _hidden "/Game/Meshes/Noise100.Noise100"))
    (:NewEnumerator4
      (Components|StaticMesh|SetStaticMesh (Variables|Default|GetRepresentation) "/Game/Meshes/Noise150.Noise150")
      (Components|StaticMesh|SetStaticMesh _hidden "/Game/Meshes/Noise150.Noise150"))))